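; BL_Storm is a launcher helper library that shows error and notification popups as UMG widgets on top of the viewport.
; Print Error spawns WB_Error from an error struct when HasError is set, passing its code, name and joined message and details.
; The custom error and notification variants take a plain message and name, creating WB_Error or WB_Notification at a very high Z-order.
; Print Plashka is an empty stub.
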(fn `Print Error`
  (params (Error :type "PlayFabError Structure"))
  (bind (_haserror _errorcode _errorname _errormessage _errordetails) (break `PlayFabError` Error))
  (if _haserror
    (bind _returnvalue (`|CreateWidget` "/Game/Launcher/UI/Desktop/Notifications/WB_Error.WB_Error_C" null _errorcode (`KismetStringLibrary.Concat_StrStr` _errormessage " \n" _errordetails) _errorname))
    (`UserWidget.AddToViewport` _returnvalue 999999999)))

(fn `Print Error (Custom)`
  (params (Message :type String) (Name :type String))
  (bind _returnvalue (`|CreateWidget` "/Game/Launcher/UI/Desktop/Notifications/WB_Error.WB_Error_C" null 0 Message Name))
  (`UserWidget.AddToViewport` _returnvalue 999999999))

(fn `Print Notification`
  (params (Message :type String) (Name :type String))
  (bind _returnvalue (`|CreateWidget` "/Game/Launcher/UI/Desktop/Notifications/WB_Notification.WB_Notification_C" null Message Name))
  (`UserWidget.AddToViewport` _returnvalue 999999999))

(fn `Print Plashka`)