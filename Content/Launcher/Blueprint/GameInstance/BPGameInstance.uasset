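; Game instance Blueprint for the launcher that holds the install directory and auto-update setting.
; On Init it reads both values by fixed line index from a text config file at a hardcoded absolute C: path, turning the "True" string into the AutoUpdates boolean.
; A self-recalling custom event prints AutoUpdates every few seconds as debug output, though nothing in this graph starts it.
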(event `self.ReceiveInit`
  (bind _filecontent (`FileSystemLibraryBPLibrary.LoadTextFileToStringArray` "C:\\Reverse\\configs\\data\\data.txt"))
  (set `self.InstallDirectory` (`|GetArrayItem` _filecontent 11))
  (if (`KismetStringLibrary.EqualEqual_StrStr` (`|GetArrayItem` _filecontent 8) "True")
    (set `self.bAutoUpdates` true)
    (else
      (set `self.bAutoUpdates` false))))

(event `CustomEvent`
  (`KismetSystemLibrary.PrintString` (select `bool` (`self.bAutoUpdates`) :`false` "False" :`true` "True"))
  (`KismetSystemLibrary.Delay` 3.0)
  (`self.CustomEvent`))